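; BP_Axe is a swinging axe obstacle that knocks the first-person player character away on contact.
; Each tick it sets the pitch of its PivotPoint from a sine of game time, producing a continuous pendulum swing.
; When its Box overlaps BP_FirstPersonCharacter, it launches the character along the direction from the actor's origin to the character, scaled by Force and overriding existing velocity.
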(event `self.ReceiveTick`
  (params (DeltaSeconds :type "Float (single-precision)"))
  (`SceneComponent.K2_SetRelativeRotation` (`self.PivotPoint`) (`KismetMathLibrary.MakeRotator` 0.0 (* (`KismetMathLibrary.Sin` (* (`KismetSystemLibrary.GetGameTimeInSeconds`) 2.0)) 60.0)) false false))

(event `self.Box.OnComponentBeginOverlap`
  (params (OverlappedComponent :type "PrimitiveComponent Object Reference") (OtherActor :type "Actor Object Reference") (OtherComp :type "PrimitiveComponent Object Reference") (OtherBodyIndex :type Integer) (bFromSweep :type Boolean) (SweepResult :type "HitResult Structure (by ref)"))
  (bind _asbp_first_person_character (cast `/Game/FirstPerson/Blueprints/BP_FirstPersonCharacter` OtherActor))
  (`Character.LaunchCharacter` _asbp_first_person_character (* (`KismetMathLibrary.Normal` (- (`self.K2_GetActorLocation` _asbp_first_person_character) (`self.K2_GetActorLocation`))) (`self.Force`)) true true))

(fn `UserConstructionScript`)